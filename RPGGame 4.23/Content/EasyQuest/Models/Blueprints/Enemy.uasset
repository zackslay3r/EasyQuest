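; Enemy actor for EasyQuest that takes damage from magic projectiles and feeds the player's quest and leveling systems when killed.
; Each MagicProjectile overlap spawns an explosion, subtracts a fixed amount of Health and destroys the projectile.
; At zero Health, Death drops a LootPickup at the foot socket, destroys the enemy and awards LevelingComponent experience.
; The overlap handler then notifies every quest in the player's QuestLog of the kill.
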(event Collision|EventActorBeginOverlap
  (params (OtherActor :type Actor%20Object%20Reference))
  ;[1 1 1] This is for allowing the AI to take damage
  (bind _asmagic_projectile (Utilities|Casting|CastToMagicProjectile OtherActor))
  (Development|PrintString "hit")
  (Effects|SpawnEmitteratLocation "/Game/StarterContent/Particles/P_Explosion.P_Explosion" (Transformation|GetActorLocation _asmagic_projectile))
  (bind _output_get (Variables|Default|SetHealth (- (Variables|Default|GetHealth) 0.5)))
  (if (<= _output_get 0.0)
    (Actor|DestroyActor _asmagic_projectile)
    (CallFunction|Death)
    (bind _asplayer (Utilities|Casting|CastToPlayer (Game|GetPlayerCharacter 0)))
    (for _array_element (Variables|/Game/EasyQuest/QuestSystem/QuestLog.QuestLog_C|GetQuests (Variables|/Game/EasyQuest/Models/Blueprints/Player/Player.Player_C|GetQuestLog _asplayer))
      (Default|CallKilledAnEnemy _array_element self))
    (else
      (Actor|DestroyActor _asmagic_projectile))))

(event EventTick
  (params (DeltaSeconds :type Float%20%28single-precision%29)))

(fn ConstructionScript)

(fn TakeDamage
  (Effects|SpawnEmitteratLocation "/Game/StarterContent/Particles/P_Explosion.P_Explosion" (Transformation|GetActorLocation)))

(fn Death
  (Game|SpawnActorfromClass "/Game/EasyQuest/Models/Blueprints/LootPickup.LootPickup_C" (Math|Transform|MakeTransform (Transformation|GetSocketLocation (Variables|Character|GetMesh) "foot_l")) "Undefined" 0 0)
  (Actor|DestroyActor)
  (Utilities|RewardKillExperience))