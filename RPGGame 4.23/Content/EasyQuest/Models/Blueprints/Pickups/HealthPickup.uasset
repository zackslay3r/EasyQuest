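; HealthPickup is a pickup actor that heals the player on overlap.
; When the overlapping actor casts to Player and its Health is not above full, it adds a fixed fraction of health and clamps the result to the maximum.
; It then spawns the heal potion particle effect at the player's location and destroys itself, even if the player was already exactly at full health.
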(event EventBeginPlay)

(event Collision|EventActorBeginOverlap
  (params (OtherActor :type Actor%20Object%20Reference))
  ;[1 1 1] This is the code for when a player steps over a pickup, heal the player
  (bind _asplayer (Utilities|Casting|CastToPlayer OtherActor))
  (if (not (> (Variables|/Game/EasyQuest/Models/Blueprints/Player/Player.Player_C|GetHealth _asplayer) 1.0))
    (bind _output_get (Variables|/Game/EasyQuest/Models/Blueprints/Player/Player.Player_C|SetHealth _asplayer (+ (Variables|/Game/EasyQuest/Models/Blueprints/Player/Player.Player_C|GetHealth _asplayer) 0.2)))
    (if (> _output_get 1.0)
      (Variables|/Game/EasyQuest/Models/Blueprints/Player/Player.Player_C|SetHealth _asplayer 1.0))
    (Effects|SpawnEmitteratLocation "/Game/InfinityBladeEffects/Effects/FX_Ability/Heal/P_Heal_Potion.P_Heal_Potion" (Transformation|GetActorLocation _asplayer))
    (Actor|DestroyActor)))

(event EventTick
  (params (DeltaSeconds :type Float%20%28single-precision%29)))

(fn ConstructionScript)